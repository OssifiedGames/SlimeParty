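; Destructible nature prop that takes a random static mesh from a list on BeginPlay and can be destroyed by enemies or the player.
; An enemy hit or a ForceDestruction call triggers destruction only when that character has enough FoodPoints.
; Destruction disables collision, spawns smoke and a crash sound, then a timeline sinks the mesh before destroying the actor.
; Smoke is small at the enemy's location, but much larger at the prop's for player destruction.
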(event Custom|ForceDestruction
  (params (Player :type BP%20Player%20Object%20Reference))
  (|DestructionPlayer_2_2 Player))

(event Collision|EventHit
  (params (MyComp :type Primitive%20Component%20Object%20Reference) (Other :type Actor%20Object%20Reference) (OtherComp :type Primitive%20Component%20Object%20Reference) (bSelfMoved :type Boolean) (HitLocation :type Vector :default "0, 0, 0") (HitNormal :type Vector :default "0, 0, 0") (NormalImpulse :type Vector :default "0, 0, 0") (Hit :type Hit%20Result%20Structure%20%28by%20ref%29))
  (bind _asbp_enemy (Utilities|Casting|CastToBP_enemy Other))
  (|DestructionEnemy_2 _asbp_enemy))

(event EventBeginPlay
  (Components|StaticMesh|SetStaticMesh (Variables|Default|GetSM) (.OutItem (Utilities|Array|Random (Variables|Default|GetSMList)))))

(fn ConstructionScript)