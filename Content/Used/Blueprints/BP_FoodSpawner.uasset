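; BP_FoodSpawner is an actor that fills the SlimeParty game world with BP_Food pickups when play begins.
; It caches the GM_SlimeParty game mode, then spawns food at random XY points across a large square area at a fixed height.
; Each spawn increments the game mode's food counter, and a short-delay loop repeats until the cap is reached, after which it stops for good.
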(event EventBeginPlay
  (Utilities|FlowControl|Sequence
    (:then_0
      (bind _asgm_slime_party (Utilities|Casting|CastToGM_SlimeParty (Game|GetGameMode)))
      (Variables|Default|SetGameMode _asgm_slime_party))
    (:then_1
      (Utilities|IsValid (Variables|Default|GetGameMode)
        (:Is%20Valid
          (if (< (Variables|/Game/Used/Blueprints/GM_SlimeParty.GM_SlimeParty_C|GetFoodInGame (Variables|Default|GetGameMode)) 12000) :!label _label
            (Game|SpawnActorfromClass "/Game/Used/Blueprints/BP_Food.BP_Food_C" (Math|Transform|MakeTransform (Math|Vector|MakeVector (Math|Random|RandomFloatinRange -4e+05 4e+05) (Math|Random|RandomFloatinRange -4e+05 4e+05) 85.0) "0, 0, 0" "1.000000,1.000000,1.000000") "AlwaysSpawn" "MultiplyWithRoot" 0 0)
            (Math|Integer|IncrementInt (Variables|/Game/Used/Blueprints/GM_SlimeParty.GM_SlimeParty_C|GetFoodInGame (Variables|Default|GetGameMode))
              (:%20%20
                (Utilities|FlowControl|Delay 0.001)
                (goto _label)))))))))

(fn ConstructionScript)