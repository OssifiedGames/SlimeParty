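; Spawner actor that scatters destructible buildings, props and nature across a large, hard-coded map area at BeginPlay.
; Three macros run in turn, each using nested MaxLoop and MaxDestructiblesPerLoop loops to spawn its class at random XY positions and fixed height.
; Buildings and props adjust for collisions where possible but always spawn.
; Nature spawns regardless of collision and is the only category stored in the Destructibles array.
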(event EventBeginPlay
  (Utilities|FlowControl|Sequence
    (:then_0
      (|Buildings))
    (:then_1
      (|Props))
    (:then_2
      (|Nature))))

(fn ConstructionScript)