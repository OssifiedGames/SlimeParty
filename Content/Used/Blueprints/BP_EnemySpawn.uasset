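; BP_EnemySpawn is a spawn point that creates a BP_enemy at its own location when InitEnemySpawn is called.
; The spawn adjusts for collisions where possible but always happens.
; Any BP_Destructible_Buildings actors overlapping the spawn point are then destroyed, and in that case the new enemy is moved 1000 units straight up without a sweep.
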(event Custom|InitEnemySpawn
  (bind _overlappingactors (Collision|GetOverlappingActors "/Game/Used/Blueprints/BP_Destructible_Buildings.BP_Destructible_Buildings_C" :!class /Script/Engine.Actor))
  (bind _returnvalue (Game|SpawnActorfromClass "/Game/Used/Blueprints/BP_enemy.BP_enemy_C" (Math|Transform|MakeTransform (Transformation|GetActorLocation) "0, 0, 0" "1.000000,1.000000,1.000000") "AdjustIfPossibleButAlwaysSpawn" "MultiplyWithRoot" 0 0))
  (if (> (Utilities|Array|Length _overlappingactors) 0)
    (for _array_element _overlappingactors
      (Actor|DestroyActor _array_element))
    (Transformation|SetActorLocation _returnvalue (+ (Transformation|GetActorLocation _returnvalue) "0.000000,0.000000,1000.000000") false false)))

(fn ConstructionScript)