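; BP_Food is a food actor that randomly becomes a low, mid or high tier on BeginPlay, with higher tiers rarer.
; The tier sets its particle template, point value, pickup effect and pickup sound.
; It then destroys itself if its location fails the AI location check, or if it overlaps a destructible building after a short delay, cleaning up bad spawns.
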(event EventBeginPlay
  (Utilities|FlowControl|Sequence
    (:then_0
      (bind _output_get (Variables|Default|SetFoodTierIndex (Math|Random|RandomIntegerinRange 1 100)))
      (if (<= _output_get 65)
        (Effects|Components|ParticleSystem|SetTemplate (Variables|Default|GetP_Projectile_Bomb01Blue) "/Game/Used/P_Food_Low.P_Food_Low")
        (Variables|Default|SetFoodPoints 0.1)
        (Variables|Default|SetFX_Pickup "/Game/Used/P_Hit_Food_Low.P_Hit_Food_Low")
        (Variables|Default|SetPickupSound "/Game/Used/Food_Low_FX.Food_Low_FX")
        (elif (<= _output_get 90)
          (Effects|Components|ParticleSystem|SetTemplate (Variables|Default|GetP_Projectile_Bomb01Blue) "/Game/Used/P_Food_Mid.P_Food_Mid")
          (Variables|Default|SetFoodPoints 0.5)
          (Variables|Default|SetFX_Pickup "/Game/Used/P_Hit_Food_Mid.P_Hit_Food_Mid")
          (Variables|Default|SetPickupSound "/Game/Used/Food_Mid_FX.Food_Mid_FX")
          (else
            (Effects|Components|ParticleSystem|SetTemplate (Variables|Default|GetP_Projectile_Bomb01Blue) "/Game/Used/P_Food_High.P_Food_High")
            (Variables|Default|SetFoodPoints 1.0)
            (Variables|Default|SetFX_Pickup "/Game/Used/P_Hit_Food_High.P_Hit_Food_High")
            (Variables|Default|SetPickupSound "/Game/Used/Food_High_FX.Food_High_FX")))))
    (:then_1
      (if (not (AI|IsValidAILocation (Transformation|GetActorLocation)))
        (Actor|DestroyActor)))
    (:then_2
      (Utilities|FlowControl|Delay 3.0)
      (if (> (Utilities|Array|Length (Collision|GetOverlappingActors "/Game/Used/Blueprints/BP_Destructible_Buildings.BP_Destructible_Buildings_C" :!class /Script/Engine.Actor)) 0)
        (Actor|DestroyActor)))))

(fn ConstructionScript)