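; AI slime enemy for Slime Party that grows by absorbing food and smaller enemies, and is handed to a bigger player to eat.
; Sphere overlaps resolve eating, with FoodPoints driving scale, label and slower animation, plus food-tiered effects and camera shake.
; An Overlap volume, held at fixed world scale, flags smaller nearby players or enemies.
; BeginPlay randomises material, colours and starting points, and starts the floating arrow timeline.
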(event OnComponentBeginOverlap(Overlap)
  (params (OverlappedComponent :type Primitive%20Component%20Object%20Reference) (OtherActor :type Actor%20Object%20Reference) (OtherComp :type Primitive%20Component%20Object%20Reference) (OtherBodyIndex :type Integer) (bFromSweep :type Boolean) (SweepResult :type Hit%20Result%20Structure%20%28by%20ref%29))
  (bind _asbp_player (Utilities|Casting|CastToBP_Player OtherActor)
    (:then
      (if (< (Variables|/Game/Used/Blueprints/BP_Player.BP_Player_C|GetFood%20Points _asbp_player) (Variables|Default|GetFood%20Points))
        (Variables|Default|SetNearPlayer true)))
    (:CastFailed
      (bind _asbp_enemy (Utilities|Casting|CastToBP_enemy OtherActor))
      (if (< (Variables|BP_enemy_C|GetFood%20Points _asbp_enemy) (Variables|Default|GetFood%20Points))
        (Variables|Default|SetNearAI true)
        (Variables|Default|SetAI _asbp_enemy)))))

(event OnComponentEndOverlap(Overlap)
  (params (OverlappedComponent :type Primitive%20Component%20Object%20Reference) (OtherActor :type Actor%20Object%20Reference) (OtherComp :type Primitive%20Component%20Object%20Reference) (OtherBodyIndex :type Integer))
  (Utilities|Casting|CastToBP_Player OtherActor
    (:then
      (Variables|Default|SetNearPlayer false))
    (:CastFailed
      (bind _asbp_enemy (Utilities|Casting|CastToBP_enemy OtherActor))
      (Variables|Default|SetNearAI false)
      (Variables|Default|SetAI _asbp_enemy))))

(event OnComponentBeginOverlap(Sphere)
  (params (OverlappedComponent :type Primitive%20Component%20Object%20Reference) (OtherActor :type Actor%20Object%20Reference) (OtherComp :type Primitive%20Component%20Object%20Reference) (OtherBodyIndex :type Integer) (bFromSweep :type Boolean) (SweepResult :type Hit%20Result%20Structure%20%28by%20ref%29))
  (|AbsorbEnemy_2_2 OtherActor
    (:CastFailed
      (bind _asbp_food (Utilities|Casting|CastToBP_Food OtherActor)
        (:then
          (Utilities|IsValid _asbp_food
            (:Is%20Valid
              (Variables|Default|SetAs%20BP%20Food _asbp_food)
              (bind _output_get (Variables|Default|SetFood%20Points (+ (Variables|/Game/Used/Blueprints/BP_Food.BP_Food_C|GetFoodPoints _asbp_food) (Variables|Default|GetFood%20Points))))
              (Transformation|SetActorScale3D (Math|Conversions|ToVector(Float) _output_get))
              (Transformation|SetWorldScale3D (Variables|Default|GetOverlap) "500.000000,500.000000,500.000000")
              (CallFunction|AnimHandling)
              (|FX_2_2 (Variables|/Game/Used/Blueprints/BP_Food.BP_Food_C|GetFX_Pickup _asbp_food))
              (|Shakedeterm_2 (Variables|/Game/Used/Blueprints/BP_Food.BP_Food_C|GetFX_Pickup _asbp_food)
                (:NewParam
                  (Actor|DestroyActor _asbp_food)
                  (Camera|PlayWorldCameraShake (Variables|Default|GetShakeType) (Transformation|GetActorLocation) 1e+02 1e+03)
                  (Math|Integer|DecrementInt (Variables|/Game/Used/Blueprints/GM_SlimeParty.GM_SlimeParty_C|GetFoodInGame (Variables|Default|GetGameMode))
                    (:%20%20
                      (Rendering|Components|TextRender|SetText (Variables|Default|GetPoints) (Utilities|Text|ToText(Float) (Variables|Default|GetFood%20Points) "HalfToEven")))))))))
        (:CastFailed
          (bind _asbp_player (Utilities|Casting|CastToBP_Player OtherActor))
          (if (< (Variables|Default|GetFood%20Points) (Variables|/Game/Used/Blueprints/BP_Player.BP_Player_C|GetFood%20Points _asbp_player))
            (Default|ForceEating _asbp_player self (Variables|Default|GetFood%20Points))))))))

(event Custom|ForceScaleUpdate
  (CallFunction|SetPoints)
  (Transformation|SetActorScale3D (Math|Conversions|ToVector(Float) (Variables|Default|GetFood%20Points)))
  (Transformation|SetWorldScale3D (Variables|Default|GetOverlap) "500.000000,500.000000,500.000000"))

(event EventBeginPlay
  (Utilities|FlowControl|Sequence
    (:then_0
      (bind _returnvalue (Rendering|Material|CreateDynamicMaterialInstance (.OutItem (Utilities|Array|Random (Variables|Default|GetPossibleMaterials))) "None" "None" :!class /Script/Engine.KismetMaterialLibrary))
      (bind _output_get (Variables|Default|SetMyDynaMat _returnvalue))
      (Variables|Default|SetParameter%20Name "Dirt Color")
      (CallFunction|SetColor (Variables|Default|GetParameter%20Name) _output_get)
      (Variables|Default|SetParameter%20Name "Eyes color")
      (CallFunction|SetColor (Variables|Default|GetParameter%20Name) (Variables|Default|GetMyDynaMat))
      (Variables|Default|SetParameter%20Name "inner color")
      (CallFunction|SetColor (Variables|Default|GetParameter%20Name) (Variables|Default|GetMyDynaMat))
      (Variables|Default|SetParameter%20Name "outer collor")
      (CallFunction|SetColor (Variables|Default|GetParameter%20Name) (Variables|Default|GetMyDynaMat))
      (Rendering|Material|SetMaterial (Variables|Character|GetMesh) 0 (Variables|Default|GetMyDynaMat))
      (bind _asgm_slime_party (Utilities|Casting|CastToGM_SlimeParty (Game|GetGameMode)))
      (Variables|Default|SetGameMode _asgm_slime_party)
      (Actor|GetAllActorsOfClass "/Script/Engine.TriggerBase")
      (Variables|Default|SetFood%20Points (Math|Conversions|ToFloat(Integer) (Math|Float|Round (Math|Random|RandomFloatinRange 1.0 5e+01))))
      (CallFunction|ForceScaleUpdate))
    (:then_1
      (bind _floating (Timeline|ArrowFloat PlayFromStart)
        (:Update
          (Transformation|AddWorldOffset (Variables|Default|GetControlRig_Arrow_solid) (Math|Vector|MakeVector 0.0 0.0 _floating) false false))))))

(fn ConstructionScript)

(fn SetColor
  (params (ParameterName :type Name) (Mat :type Material%20Instance%20Dynamic%20Object%20Reference))
  (Rendering|Material|SetVectorParameterValue Mat ParameterName (Utilities|Struct|MakeLinearColor (Math|Random|RandomFloatinRange 0.0 1.0) (Math|Random|RandomFloatinRange 0.0 1.0) (Math|Random|RandomFloatinRange 0.0 1.0) 1.0) :!class /Script/Engine.MaterialInstanceDynamic))

(fn SetPoints
  (Rendering|Components|TextRender|SetText (Variables|Default|GetPoints) (Utilities|Text|ToText(Float) (Variables|Default|GetFood%20Points) "HalfToEven")))

(fn AnimHandling
  (|Handling_2))