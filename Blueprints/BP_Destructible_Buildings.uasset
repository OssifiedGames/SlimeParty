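; Destructible building actor that collapses when a player or enemy with enough FoodPoints destroys it.
; On BeginPlay it picks a random mesh, then after a short delay destroys any BP_Food overlapping it.
; Enemies trigger destruction by hitting it, while players go through ForceDestruction with a higher threshold.
; Destruction disables collision, plays smoke and sound, and sinks the mesh on a Timeline before destroying the actor.
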(event Custom|ForceDestruction
  (params (Player :type BP%20Player%20Object%20Reference))
  (|DestructionPlayer Player))

(event Collision|EventHit
  (params (MyComp :type Primitive%20Component%20Object%20Reference) (Other :type Actor%20Object%20Reference) (OtherComp :type Primitive%20Component%20Object%20Reference) (bSelfMoved :type Boolean) (HitLocation :type Vector :default "0, 0, 0") (HitNormal :type Vector :default "0, 0, 0") (NormalImpulse :type Vector :default "0, 0, 0") (Hit :type Hit%20Result%20Structure%20%28by%20ref%29))
  (bind _asbp_enemy (Utilities|Casting|CastToBP_enemy Other))
  (|DestructionEnemy _asbp_enemy))

(event EventBeginPlay
  (bind _overlappingactors (Collision|GetOverlappingActors "/Game/Used/Blueprints/BP_Food.BP_Food_C" :!class /Script/Engine.Actor))
  (Components|StaticMesh|SetStaticMesh (Variables|Default|GetSM) (.OutItem (Utilities|Array|Random (Variables|Default|GetSMList))))
  (Utilities|FlowControl|Delay 2.0)
  (if (> (Utilities|Array|Length _overlappingactors) 0)
    (bind _output_get (Variables|Default|SetFoodToDestroy _overlappingactors))
    (for _array_element _output_get
      (Actor|DestroyActor _array_element))))

(fn ConstructionScript)